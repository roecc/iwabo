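; Game mode for the Inkpot adventure demo that puts the story display on screen and connects it to Inkpot story events.
; On BeginPlay it creates the adventure display widget, gives it focus in Game and UI input mode with the cursor visible, and binds to Inkpot's story begin and end events.
; Story begin passes the story to the widget to show, while the story end handler is an empty stub.
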(event Custom|Event%20OnStoryBegin
  (params (Story :type Inkpot%20Story%20Object%20Reference))
  ;[1 1 1] Display story when it begins
  (Class|InkpotDemoWidget|ShowStory (Variables|Default|GetStoryDisplay) Story))

(event Custom|Event%20OnStoryEnd
  (params (Story :type Inkpot%20Story%20Object%20Reference))
  ;[1 1 1] Story End
)

(event EventBeginPlay
  (bind _returnvalue (Game|GetPlayerController 0))
  (bind _returnvalue_2 (|Inkpot))
  ;[1 1 1] Setup display and control
  (bind _returnvalue_3 (UserInterface|CreateWidget "/Game/InkpotDemo/UI/WBP_Display_Adventure.WBP_Display_Adventure_C"))
  (bind _output_get (Variables|Default|SetStoryDisplay _returnvalue_3))
  (UserInterface|Viewport|AddtoViewport _output_get 0)
  (Input|SetInputModeGameandUI _returnvalue (Variables|Default|GetStoryDisplay) "DoNotLock" false false)
  (Variables|/Script/Engine.PlayerController|SetbShowMouseCursor _returnvalue true)
  ;[1 1 1] Bind Inkpot events
  (EventDispatchers|AssignEventonStoryBegin _returnvalue_2 (delegate Custom|Event%20OnStoryBegin))
  (EventDispatchers|AssignEventonStoryEnd _returnvalue_2 (delegate Custom|Event%20OnStoryEnd)))

(fn ConstructionScript)