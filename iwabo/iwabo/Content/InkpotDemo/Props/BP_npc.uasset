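; Demo NPC actor that teleports between the garden, living room and parent bedroom to follow the Ink story's "mary_ann" location list.
; On BeginPlay it hooks Inkpot's story-begin event, then re-reads the list whenever story JSON is loaded.
; An Ink watch component also passes variable changes to UpdateLocation.
; UpdateLocation maps the list item to a hardcoded position, disabling collision during the teleport.
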(event EventonVariableChange(InkWatchMA)
  (params (Story :type Inkpot%20Story%20Object%20Reference) (Variable :type String) (NewValue :type Inkpot%20Value%20Structure%20%28by%20ref%29))
  (CallFunction|UpdateLocation NewValue))

(event Custom|OnStoryBegin
  (params (Story :type Inkpot%20Story%20Object%20Reference))
  (EventDispatchers|AssignEventonStoryLoadJSON Story (delegate Custom|OnStoryLoadJSON)))

(event Custom|OnStoryLoadJSON
  (params (Story :type Inkpot%20Story%20Object%20Reference))
  (CallFunction|UpdateLocation (.ReturnValue (Class|InkpotStory|GetList Story "mary_ann"))))

(event EventBeginPlay
  (EventDispatchers|BindEventtoEventonStoryBegin (|Inkpot) (delegate Custom|OnStoryBegin)))

(fn ConstructionScript)

(fn UpdateLocation
  (params (Value :type Inkpot%20Value%20Structure%20%28by%20ref%29))
  (bind _returnvalue (Class|InkpotValueLibrary|InkpotValueasList Value))
  (Collision|SetActorEnableCollision false)
  (if (Class|InkpotListLibrary|ContainsItem _returnvalue "location.garden")
    (Transformation|SetActorLocation (Math|Vector|MakeVector -1e+03 -5.2e+02 0.0) false true)
    (elif (Class|InkpotListLibrary|ContainsItem _returnvalue "location.living_room")
      (Transformation|SetActorLocation (Math|Vector|MakeVector -1e+03 -1.5e+03 0.0) false true)
      (elif (Class|InkpotListLibrary|ContainsItem _returnvalue "location.parent_bedroom")
        (Transformation|SetActorLocation (Math|Vector|MakeVector -1e+03 -1e+03 0.0) false true))))
  (Collision|SetActorEnableCollision true))