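; Actor component that keeps its owning interactable in sync with an Ink story list variable.
; On BeginPlay it gets the variable name through the owner's BPI_Interactable interface and binds to the GameInstance's story init and JSON load events.
; Story init registers an Ink variable observer and binds the OnVarChange dispatcher.
; Variable changes and story loads fire that dispatcher, which passes the current list value to the owner's UpdateState.
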(event Custom|Bound_GI_Init
  (params (Story :type Inkpot%20Story%20Object%20Reference))
  (Class|InkpotStory|SetonVariableChange Story (delegate Custom|Bound_Ink_OnVariableChange) (Variables|Default|GetVarName))
  (EventDispatchers|BindEventtoOnVarChange (delegate Custom|Bound_OnVarChange)))

(event Custom|Bound_Ink_OnVariableChange
  (params (Story :type Inkpot%20Story%20Object%20Reference) (Variable :type String) (NewValue :type Inkpot%20Value%20Structure%20%28by%20ref%29))
  (Default|CallOnVarChange Story Variable))

(event Custom|Bound_GI_OnStoryLoad
  (params (Story :type Inkpot%20Story%20Object%20Reference))
  (Default|CallOnVarChange Story (Variables|Default|GetVarName)))

(event Custom|Bound_OnVarChange
  (params (Stoy :type Inkpot%20Story%20Object%20Reference) (VarName :type String))
  (if (Utilities|IsValidInterface (Variables|Default|GetI_Interactable))
    (Default|UpdateState (Variables|Default|GetI_Interactable) Stoy VarName (.ReturnValue (Class|InkpotStory|GetList Stoy (Variables|Default|GetVarName))))
    (else
      (Development|PrintString "INVALID INTERFACE"))))

(event EventBeginPlay
  (bind _self self)
  (bind _game (CallFunction|GetGameInstance _self))
  (EventDispatchers|BindEventtoOnStoryInit _game (delegate Custom|Bound_GI_Init))
  (EventDispatchers|BindEventtoOnStoryLoadJSON _game (delegate Custom|Bound_GI_OnStoryLoad))
  (bind _asbpi_interactable (Utilities|Casting|CastToBPI_Interactable (Components|GetOwner))
    (:then
      (bind _output_get (Variables|Default|SetI_Interactable _asbpi_interactable))
      (bind _varname (Default|GetInkVarName _output_get))
      (Variables|Default|SetVarName _varname))
    (:CastFailed
      (Development|PrintString "CAST FAILED"))))

(event EventTick
  (params (DeltaSeconds :type Float%20%28single-precision%29)))