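; Base NPC whose location and animation state are driven by an Ink story (Inkpot).
; On story init it passes the story and its InkName variable to the unarmed AnimBP.
; UpdateState sets the AnimBP's Ink state and resolves the location through BP_LocationServive.
; GoTo snaps to the navmesh, walks there, then teleports to the exact transform even if the move fails; FollowPlayer chases the player while SeingPawn is set.
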(event Custom|FollowPlayer
  (if (Variables|Default|GetbSeingPawn?)
    (AI|AIMoveTo self "0, 0, 0" (Game|GetPlayerCharacter 0) 1.0 false)))

(event Custom|GoTo
  (params (Destination :type Vector) (Rotation :type Rotator))
  (Transformation|SetActorLocationAndRotation (.ProjectedLocation (AI|Navigation|ProjectPointtoNavigation (Transformation|GetActorLocation) 0 0 "100.000000,100.000000,100.000000")) "0, 0, 0" false true)
  (AI|AIMoveTo self Destination 0 4.0 true
    (:OnSuccess
      _)
    (:OnFail
      _))
  (Transformation|SetActorLocationAndRotation Destination Rotation false true))

(event Custom|OnStoryLoad
  (params (Story :type Inkpot%20Story%20Object%20Reference)))

(event Custom|OnStoryInit
  (params (Story :type Inkpot%20Story%20Object%20Reference))
  (bind _inkname (Variables|Default|GetInkName))
  (if (.bSuccess (Class|InkpotStory|GetList Story _inkname))
    (Default|InkInit (Variables|Default|GetAnimInstance) Story _inkname)
    (else
      (Development|PrintString "ERROR: Couldnt set State in NPC_BASE"))))

(event EventBeginPlay
  (bind _asabp_unarmed_iwabo (Utilities|Casting|CastToABP_Unarmed_IWABO (Components|SkeletalMesh|GetAnimInstance (Variables|Character|GetMesh))))
  (Variables|Default|SetAnimInstance _asabp_unarmed_iwabo)
  (EventDispatchers|BindEventtoOnStoryInit (CallFunction|GetGameInstance self) (delegate Custom|OnStoryInit)))

(event Collision|EventActorBeginOverlap
  (params (OtherActor :type Actor%20Object%20Reference)))

(event EventTick
  (params (DeltaSeconds :type Float%20%28single-precision%29)))

(event EventUpdateState
  (params (Story :type Inkpot%20Story%20Object%20Reference) (VarName :type String) (Value :type Inkpot%20Value%20Structure))
  (CallFunction|UpdateLocation Story "location" Value)
  (Variables|/Game/IWABO/TMP/ABP_Unarmed_IWABO.ABP_Unarmed_IWABO_C|SetInkState (Variables|Default|GetAnimInstance) (Class|InkpotValueLibrary|InkpotValueasList Value)))

(event EventOnInteract)

(fn ConstructionScript)

(fn UpdateLocation
  (params (Story :type Inkpot%20Story%20Object%20Reference) (Variable :type String) (Value :type Inkpot%20Value%20Structure%20%28by%20ref%29))
  (bind _returnvalue (Actor|GetActorOfClass "/Game/IWABO/TMP/BP_LocationServive.BP_LocationServive_C"))
  (if (Utilities|Operators|EqualEqual :A (.Rotation (Default|GetLocation _returnvalue Story Value)) :ErrorTolerance 0.1)
    _
    (else
      _))
  (CallFunction|Goto (.Location (Default|GetLocation _returnvalue Story Value)) (.Rotation (Default|GetLocation _returnvalue Story Value))))

(fn Var^List
  (params (Story :type Inkpot%20Story%20Object%20Reference) (list :type String) (Var :type Inkpot%20Value%20Structure%20%28by%20ref%29))
  (return (.RightS (Utilities|String|Split (Class|InkpotListLibrary|ToString (Class|InkpotListLibrary|Intersect (Class|InkpotValueLibrary|InkpotValueasList Var) (.ReturnValue (Class|InkpotStory|GetList Story list))) true) "."))))

(fn GetInkVarName
  (return (Variables|Default|GetInkName)))