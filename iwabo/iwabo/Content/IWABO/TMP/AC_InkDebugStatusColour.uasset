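; Debug actor component that tints a mesh to show the maintenance and repair state held in an Ink story variable.
; On BeginPlay it puts a dynamic material on the owner's mesh, or that of its AC_Interactable's ObjectRef, and binds to AC_WatchInk's change event.
; Each change reads the Inkpot list: repair state picks red, yellow or green, and maintain state scales brightness from forgotten to loved.
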(event Custom|Bound_InkWatch_OnVarChange
  (params (Stoy :type Inkpot%20Story%20Object%20Reference) (VarName :type String))
  (CallFunction|SetColourfromVar Stoy VarName))

(event EventBeginPlay
  (bind _returnvalue (Components|GetOwner))
  (bind _returnvalue_2 (Components|GetOwner))
  (bind _returnvalue_3 (Actor|GetComponentbyClass _returnvalue_2 "/Game/IWABO/TMP/AC_WatchInk.AC_WatchInk_C"))
  (bind _returnvalue_4 (Actor|GetComponentbyClass _returnvalue "/Game/IWABO/TMP/AC_Interactable.AC_Interactable_C"))
  (bind _returnvalue_5 (Actor|GetComponentbyClass _returnvalue "/Script/Engine.MeshComponent"))
  (bind _objectref (Variables|/Game/IWABO/TMP/AC_Interactable.AC_Interactable_C|GetObjectRef _returnvalue_4))
  (bind _returnvalue_6 (Actor|GetComponentbyClass _objectref "/Script/Engine.MeshComponent"))
  (Utilities|IsValid _returnvalue_5
    (:Is%20Valid
      (Variables|Default|SetMesh _returnvalue_5)
      (bind _returnvalue_7 (Rendering|Material|CreateDynamicMaterialInstance (Variables|Default|GetMesh) 0 "/Engine/BasicShapes/BasicShapeMaterial_Inst.BasicShapeMaterial_Inst" "None" :!class /Script/Engine.PrimitiveComponent :!label _label))
      (Variables|Default|SetMaterial _returnvalue_7)
      (Utilities|IsValid _returnvalue_3
        (:Is%20Valid
          (EventDispatchers|BindEventtoOnVarChange _returnvalue_3 (delegate Custom|Bound_InkWatch_OnVarChange))
          (Development|PrintString "Hurray"))
        (:Is%20Not%20Valid
          (Development|PrintString "ERROR: AC_StatusColour without InkWatch!")
          (Components|Activation|SetActive false false))))
    (:Is%20Not%20Valid
      (Utilities|IsValid _objectref
        (:Is%20Valid
          (Utilities|IsValid _returnvalue_6
            (:Is%20Valid
              (Variables|Default|SetMesh _returnvalue_6)
              (goto _label))))
        (:Is%20Not%20Valid
          (Development|PrintString "NOT FOUND"))))))

(event EventTick
  (params (DeltaSeconds :type Float%20%28single-precision%29)))

(fn SetColourfromVar
  (params (Story :type Inkpot%20Story%20Object%20Reference) (Variable :type String))
  (bind _returnvalue (Class|InkpotStory|GetList Story Variable))
  (bind _returnvalue_2 (Class|InkpotValueLibrary|InkpotValueasList _returnvalue))
  (Utilities|FlowControl|Sequence
    (:then_0
      (if (Class|InkpotListLibrary|ContainsItem _returnvalue_2 "maintain_state.forgotten")
        (LocalVariables|SetMult 0.2)
        (elif (Class|InkpotListLibrary|ContainsItem _returnvalue_2 "maintain_state.neglected")
          (LocalVariables|SetMult 0.4)
          (elif (Class|InkpotListLibrary|ContainsItem _returnvalue_2 "maintain_state.maintained")
            (LocalVariables|SetMult 0.6)
            (elif (Class|InkpotListLibrary|ContainsItem _returnvalue_2 "maintain_state.well_maintained")
              (LocalVariables|SetMult 0.8)
              (elif (Class|InkpotListLibrary|ContainsItem _returnvalue_2 "maintain_state.loved")
                (LocalVariables|SetMult 1.0)))))))
    (:then_1
      (if (Class|InkpotListLibrary|ContainsItem _returnvalue_2 "repair_state.broken")
        (CallFunction|SetMeshColour "1.000000,0.000000,0.000000" (LocalVariables|GetMult))
        (elif (Class|InkpotListLibrary|ContainsItem _returnvalue_2 "repair_state.damaged")
          (CallFunction|SetMeshColour "1.000000,1.000000,0.000000" (LocalVariables|GetMult))
          (elif (Class|InkpotListLibrary|ContainsItem _returnvalue_2 "repair_state.fine")
            (CallFunction|SetMeshColour "0.000000,1.000000,0.000000" (LocalVariables|GetMult))))))))

(fn SetMeshColour
  (params (RGB :type Vector) (Mult :type Float%20%28double-precision%29))
  (bind _returnvalue (* RGB Mult))
  (bind (_x _y _z) (Math|Vector|BreakVector _returnvalue))
  (Rendering|Material|SetVectorParameterValue (Variables|Default|GetMaterial) "Color" (Utilities|Struct|MakeLinearColor _x _y _z 1.0) :!class /Script/Engine.MaterialInstanceDynamic))