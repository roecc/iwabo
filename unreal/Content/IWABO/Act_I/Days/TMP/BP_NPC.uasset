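; NPC actor that plays passive Ink conversations through Inkpot when its box is overlapped and the story's IsActive flag is false.
; Each line splits into a speaker tag and text, shown on a random tagged BP_NPC's text view after blanking the previous one.
; Lines advance on a short delay or the E key.
; Choice display is a stub, and the flow-switch and JSON-load handlers lead to an empty event.
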(event OnComponentBeginOverlap(Box)
  (params (OverlappedComponent :type Primitive%20Component%20Object%20Reference) (OtherActor :type Actor%20Object%20Reference) (OtherComp :type Primitive%20Component%20Object%20Reference) (OtherBodyIndex :type Integer) (bFromSweep :type Boolean) (SweepResult :type Hit%20Result%20Structure%20%28by%20ref%29))
  (Development|PrintString "Hello")
  (bind _returnvalue (Class|Inkpot|BeginStory (|Inkpot) (Variables|Default|GetInkStory)))
  (bind _output_get (Variables|Default|SetStory _returnvalue))
  (if (.bSuccess (Class|InkpotStory|GetBool _output_get "IsActive"))
    (if (not (.ReturnValue (Class|InkpotStory|GetBool _output_get "IsActive")))
      (Development|PrintString "This is a passive conversation!!")
      (CallFunction|OnShowStory (Variables|Default|GetStory)))))

(event Custom|OnShowStory
  (params (Story :type Inkpot%20Story%20Object%20Reference))
  (bind _output_get (Variables|Default|SetStory Story))
  (EventDispatchers|BindEventtoEventonContinue _output_get (delegate Custom|OnContinuePassive))
  (EventDispatchers|BindEventtoEventonMakeChoice (Variables|Default|GetStory) (delegate Custom|OnMakeChoice))
  (EventDispatchers|BindEventtoEventonSwitchFlow (Variables|Default|GetStory) (delegate Custom|OnSwitchFlow))
  (EventDispatchers|BindEventtoEventonStoryLoadJSON (Variables|Default|GetStory) (delegate Custom|OnLoadJSON))
  (CallFunction|ContinueifYouCan (Variables|Default|GetStory))
  (CallFunction|WaitandContinue 3.0))

(event Custom|OnContinuePassive
  (params (Story :type Inkpot%20Story%20Object%20Reference))
  (CallFunction|UpdateTextView Story)
  (bind _bhaschoices (CallFunction|UpdateChoicesView Story))
  (if _bhaschoices
    _
    (else
      _))
  (CallFunction|WaitandContinue 3.0))

(event Custom|OnMakeChoice
  (params (Story :type Inkpot%20Story%20Object%20Reference) (Choice :type Inkpot%20Choice%20Object%20Reference))
  (bind _bdidcontinue (CallFunction|ContinueifYouCan Story))
  (if _bdidcontinue
    _))

(event Custom|OnSwitchFlow
  (params (Story :type Inkpot%20Story%20Object%20Reference) (Flow :type String))
  (CallFunction|OnContinue Story))

(event Custom|OnLoadJSON
  (params (Story :type Inkpot%20Story%20Object%20Reference))
  (CallFunction|OnContinue Story))

(event Custom|OnContinue
  (params (Story :type Inkpot%20Story%20Object%20Reference)))

(event Custom|WaitAndContinue
  (params (Time :type Float%20%28single-precision%29))
  (Development|PrintString "3 sedoends latoer")
  (Utilities|FlowControl|Delay 1.0)
  (bind _bdidcontinue (CallFunction|ContinueifYouCan (Variables|Default|GetStory)))
  (if (not _bdidcontinue)
    (Rendering|Components|TextRender|SetText (Variables|Default|GetTextView) (Utilities|Text|ToText(String) (Utilities|String|Append "" "")))))

(event Collision|EventActorBeginOverlap
  (params (OtherActor :type Actor%20Object%20Reference)))

(event EventTick
  (params (DeltaSeconds :type Float%20%28single-precision%29)))

(event Input|KeyboardEvents|E
  (params (Key :type Key%20Structure :default "None"))
  (:Pressed
    (bind _bdidcontinue (CallFunction|ContinueifYouCan (Variables|Default|GetStory)))
    (if (not _bdidcontinue)
      (Rendering|Components|TextRender|SetText (Variables|Default|GetTextView) (Utilities|Text|ToText(String) (Utilities|String|Append "" ""))))))

(fn ConstructionScript)

(fn ContinueifYouCan
  (params (Story :type Inkpot%20Story%20Object%20Reference))
  (if (Class|InkpotStory|CanContinue Story)
    (Class|InkpotStory|Continue Story)
    (return true)
    (else
      (return false))))

(fn UpdateTextView
  (params (Story :type Inkpot%20Story%20Object%20Reference))
  (bind _returnvalue (Class|InkpotStory|GetCurrentText Story))
  (bind (_lefts _rights) (Utilities|String|Split _returnvalue " "))
  (bind _outactors (Actor|GetAllActorsOfClasswithTag "BP_NPC_C" (Utilities|String|StringToName _lefts)))
  (Utilities|IsValid (Variables|Default|GetLastText)
    (:Is%20Valid
      (Rendering|Components|TextRender|SetText (Variables|Default|GetLastText) (Utilities|Text|ToText(String) "")))
    (:Is%20Not%20Valid
      _))
  (Variables|Default|SetLastText (Variables|BP_NPC_C|GetTextView (.OutItem (Utilities|Array|Random _outactors))))
  (Rendering|Components|TextRender|SetText (Variables|BP_NPC_C|GetTextView (.OutItem (Utilities|Array|Random _outactors))) (Utilities|Text|ToText(String) _rights)))

(fn UpdateChoicesView
  (params (Story :type Inkpot%20Story%20Object%20Reference))
  (return false))