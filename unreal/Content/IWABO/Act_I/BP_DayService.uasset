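; BP_DayService runs the in-game day clock, from a configured start time until a configured end time.
; NewDay pulls time settings from the game instance's ConfigService, then TickTime loops through a Delay, advancing and printing the minutes.
; It also starts LS_SunCycle with play rate and start offset derived from the clock settings, so one sequence second matches one game hour.
; Reaching the end time only prints a day-over message.
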(event Custom|NewDay
  (bind _asbp_iwabo_game_instance (Utilities|Casting|CastToBP_IwaboGameInstance (Game|GetGameInstance)))
  (bind (_ticksperhour _secondsperhour _starttimeminutes _endtimeminutes) (Default|GetTimeConfig (Variables|/Game/IWABO/Core/Services/BP_IwaboGameInstance.BP_IwaboGameInstance_C|GetConfigService _asbp_iwabo_game_instance)))
  (Variables|Default|SetTicksPerHour _ticksperhour)
  (Variables|Default|SetSecondsPerHour _secondsperhour)
  (Variables|Default|SetCurrentTimeMinutes _starttimeminutes)
  (Variables|Default|SetEndTimeMinutes _endtimeminutes)
  (CallFunction|TickTime)
  (CallFunction|StartSunCycle))

(event Custom|TickTime
  (bind _ticksperhour (Variables|Default|GetTicksPerHour))
  (Utilities|FlowControl|Delay (Math|Conversions|ToFloat(Integer) (/ (Variables|Default|GetSecondsPerHour) _ticksperhour)))
  (bind _output_get (Variables|Default|SetCurrentTimeMinutes (+ (Variables|Default|GetCurrentTimeMinutes) (/ 60 _ticksperhour))))
  (Development|PrintString (Utilities|String|Append "It is now: " (Utilities|String|ToString(Integer) (/ _output_get 60)) ":" (Utilities|String|ToString(Integer) (Math|Integer|%(Integer) _output_get 60)) " O'Clock"))
  (if (>= (Variables|Default|GetCurrentTimeMinutes) (Variables|Default|GetEndTimeMinutes))
    (Development|PrintString "DAY OVER!")
    (else
      (CallFunction|TickTime))))

(event EventBeginPlay)

(fn ConstructionScript)

(fn StartSunCycle
  (bind _outactor (Sequencer|Player|CreateLevelSequencePlayer "/Game/IWABO/Act_I/LS_SunCycle.LS_SunCycle" (Utilities|Struct|MakeMovieSceneSequencePlaybackSettings true "(Value=0)" "(TickIntervalSeconds=0.000000,EvaluationBudgetMicroseconds=0.000000,bTickWhenPaused=False,bAllowRounding=True)" (/ 1.0 (Math|Conversions|ToFloat(Integer) (Variables|Default|GetSecondsPerHour))) (/ (Variables|Default|GetCurrentTimeMinutes) 60) false false false false false false "None" false)))
  (Variables|Default|SetSunSequence _outactor))