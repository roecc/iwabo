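; BP_SceneBlock is one link in a chain of NPC day-structure blocks, staging a scene with Level Sequences looked up by type.
; StartBlock resolves the NPC, falling back to BP_NPC_April, and loops one sequence until EndBlock stops it.
; Helpers relink the NextBlock chain and advance a clamped action counter.
; Walk-to-scene, which samples a sequence's NPC position while hidden, and lead-out with reverse fallback are currently disconnected.
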(event Custom|Init
  (params (NPC :type BP%20NPC%20Base%20Object%20Reference))
  (Variables|Default|SetNPC NPC))

(event Custom|OutOrRevDone
  (Default|CallOnEndBlockComplete))

(event Custom|StartBlock
  (|ValidateOrSetNPC)
  (bind _value (Utilities|FindandValidateSequence "NewEnumerator1")
    (:then
      (bind _returnvalue (Sequencer|Player|CreateLevelSequencePlayer _value (Utilities|Struct|MakeMovieSceneSequencePlaybackSettings false "(Value=0)" "(TickIntervalSeconds=0.000000,EvaluationBudgetMicroseconds=0.000000,bTickWhenPaused=False,bAllowRounding=True)" 1.0 0.0 false false false false false false "ForceRestoreState" false)))
      (Class|MovieSceneSequencePlayer|PlayLooping _returnvalue -1))))

(event Custom|PlayLoop)

(event Custom|EndBlock
  (Utilities|IsValid (stale Custom|StartBlock _returnvalue)
    (:Is%20Valid
      (Sequencer|Player|Stop (stale Custom|StartBlock _returnvalue) :!class /Script/MovieScene.MovieSceneSequencePlayer))))

(fn ConstructionScript)

(fn InjectChain
  (params (ReLink :type BP%20Scene%20Block%20Object%20Reference))
  (Utilities|IsValid (Variables|Default|GetNextBlock)
    (:Is%20Valid
      (CallFunction|InjectChain (Variables|Default|GetNextBlock) ReLink))
    (:Is%20Not%20Valid
      (Variables|Default|SetNextBlock ReLink))))

(fn SwitchChain
  (params (NextBlock :type BP%20Scene%20Block%20Object%20Reference))
  (Variables|Default|SetNextBlock NextBlock))

(fn WalktoScene
  (params (InputPin :type Level%20Sequence%20Player%20Object%20Reference))
  ;[0.15 0.15 0.15 0.5] Make NPC walk to next SceneBlock: Hides Player, loads Scene, saves location, unloads Scene, walkToSavedLoc
  (Utilities|FlowControl|Sequence
    (:then_0
      (Rendering|SetActorHiddenInGame (Variables|Default|GetNPC) true))
    (:then_1
      (Sequencer|Player|Play InputPin :!class /Script/MovieScene.MovieSceneSequencePlayer)
      (bind _output_get (LocalVariables|SetSceneLocation (.location (Transformation|GetActorTransform (Variables|Default|GetNPC)))))
      (Sequencer|Player|Stop InputPin :!class /Script/MovieScene.MovieSceneSequencePlayer))
    (:then_2
      (Rendering|SetActorHiddenInGame (Variables|Default|GetNPC) false)
      (Default|GotoScene (Variables|Default|GetNPC) _output_get self))))

(fn TryIncrementAction
  (params (Actions :type Integer))
  (bind _actionduration (Variables|Default|GetActionDuration))
  (Variables|Default|SetCurrentAction (Math|Integer|Min(Integer) (+ (Variables|Default|GetCurrentAction) Actions) (- _actionduration 1)))
  (return (- (+ (Variables|Default|GetCurrentAction) Actions) _actionduration)))

(event Custom|PlayIn
  ;[0.15 0.15 0.15 0.5] Actor has arrived, Play Lead-In Animation
)