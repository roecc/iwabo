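; BP_SurvCam is a fixed-position camera that takes over the player's view when the Iwabo third-person character enters its trigger.
; On overlap it registers itself as the character's active cam, stores it as the target, activates the camera and blends player 0's view over with ease-in.
; While active, Tick aims the camera slightly above the target's origin and sets tracking focus on it.
; GetCameraRotation exposes the camera's world rotation.
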(event OnComponentBeginOverlap(CameraTrigger)
  (params (OverlappedComponent :type Primitive%20Component%20Object%20Reference) (OtherActor :type Actor%20Object%20Reference) (OtherComp :type Primitive%20Component%20Object%20Reference) (OtherBodyIndex :type Integer) (bFromSweep :type Boolean) (SweepResult :type Hit%20Result%20Structure%20%28by%20ref%29))
  (bind _asbp_iwabo_third_person_character (Utilities|Casting|CastToBP_IwaboThirdPersonCharacter OtherActor))
  (Default|SetActiveCam _asbp_iwabo_third_person_character self)
  (CallFunction|SettoActor _asbp_iwabo_third_person_character 1.0))

(event EventBeginPlay
  (Components|Activation|SetActive (Variables|Default|GetCamera) (Variables|Default|GetbDefault?) false))

(event Collision|EventActorBeginOverlap
  (params (OtherActor :type Actor%20Object%20Reference)))

(event EventTick
  (params (DeltaSeconds :type Float%20%28single-precision%29))
  (bind _camera (Variables|Default|GetCamera))
  (bind _cameratarget (Variables|Default|GetCameraTarget))
  (bind _returnvalue (Transformation|GetActorLocation _cameratarget))
  (if (Components|Activation|IsActive (Variables|Default|GetCamera))
    (Transformation|SetWorldRotation _camera (Math|Rotator|FindLookatRotation (Transformation|GetWorldLocation (Variables|Default|GetCamera)) (Math|Vector|MakeVector (.x _returnvalue) (.y _returnvalue) (+ (.z _returnvalue) 6e+01))) false false)
    (Variables|/Script/CinematicCamera.CineCameraComponent|SetFocusSettings _camera (Utilities|Struct|MakeCameraFocusSettings "Tracking" 1e+05 (Utilities|Struct|MakeCameraTrackingFocusSettings (Utilities|ResolveSoftReference (Variables|Default|GetCameraTarget)) "0.000000,0.000000,0.000000" false) false 8.0 0.0))))

(fn ConstructionScript)

(fn SettoActor
  (params (Actor :type Actor%20Object%20Reference) (BlendTime :type Float%20%28double-precision%29))
  (Variables|Default|SetCameraTarget Actor)
  (Components|Activation|SetActive (Variables|Default|GetCamera) true false)
  (Game|Player|SetViewTargetwithBlend (Game|GetPlayerController 0) self BlendTime "VTBlend_EaseIn" 0.0 false))

(fn GetCameraRotation
  (return (Transformation|GetWorldRotation (Variables|Default|GetCamera))))