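; Base NPC Blueprint whose behavior is driven by a chain of scene blocks, starting the current block on BeginPlay.
; UpdateSceneBlock spends an action count across linked NextBlocks, then interrupts the current block and initializes the one it lands on, logging the switch.
; GoToScene walks the NPC to a destination with AIMoveTo and plays the block in on arrival.
; SetAnimation is empty, and older animation-reset logic is left unconnected.
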(event Custom|SetAnimation)

(event Custom|GoToScene
  (params (Destination :type Vector) (SceneBlock :type BP%20Scene%20Block%20Object%20Reference))
  (AI|AIMoveTo self Destination 0 5.0 false
    (:OnSuccess
      (Default|Playin SceneBlock))
    (:OnFail
      (Development|PrintString "Path Obstructed, can't reach Scene"))))

(event EventBeginPlay
  (bind _currentsceneblock (Variables|Default|GetCurrentSceneBlock))
  (Utilities|IsValid _currentsceneblock
    (:Is%20Valid
      (Default|Init _currentsceneblock self)
      (Default|StartBlock _currentsceneblock))))

(fn ConstructionScript)

(fn UpdateSceneBlock
  (params (actions :type Integer))
  (bind _currentsceneblock (Variables|Default|GetCurrentSceneBlock))
  (bind _output_get (LocalVariables|SetSceneBlock (Variables|Default|GetCurrentSceneBlock)))
  (bind _actionsleft (Default|TryIncrementAction _output_get actions))
  (bind _output_get_2 (LocalVariables|SetActionsLeft _actionsleft))
  ;[0.15 0.15 0.15 0.5] If actions still remain, begin incrementing actions on follow up scene blocks
  (if (>= _output_get_2 0)
    (while (>= (LocalVariables|GetActionsLeft) 0)
      (|IncrementBlock))
    (Utilities|IsValid (LocalVariables|GetSceneBlock)
      (:Is%20Valid
        (if (!= _currentsceneblock (LocalVariables|GetSceneBlock))
          (|LogSceneBlockUpdate)
          ;[0.15 0.15 0.15 0.5] Stop previous scene block, then start next block once done
          (EventDispatchers|BindEventtoOnPlayOutComplete _currentsceneblock (EventDispatchers|CreateEvent (LocalVariables|GetSceneBlock) :!event StartBlock))
          (Default|Interrupt _currentsceneblock)
          (Default|Init (LocalVariables|GetSceneBlock) self (Variables|Default|GetCurrentSceneBlock)))))))