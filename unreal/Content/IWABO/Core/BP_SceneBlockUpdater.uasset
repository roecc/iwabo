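; BP_SceneBlockUpdater moves an NPC through a linked chain of scene blocks as actions are spent.
; BeginPlay disables dialogue interactives on follow-up blocks and starts the current one.
; UpdateSceneBlock feeds actions to the current block, carrying leftovers along NextBlock links.
; When the resulting block differs, it logs the change, ends the current block and starts the new one; a transition sequence player is left disconnected.
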(event EventBeginPlay
  (bind _currentsceneblock (Variables|Default|GetCurrentSceneBlock))
  (Utilities|IsValid _currentsceneblock
    (:Is%20Valid
      (CallFunction|InitSceneBlocks)
      (Default|StartBlock _currentsceneblock self))))

(fn ConstructionScript)

(fn UpdateSceneBlock
  (params (actions :type Integer))
  (bind _output_get (LocalVariables|SetSceneBlock (Variables|Default|GetCurrentSceneBlock)))
  (bind _actionsleft (Default|TryIncrementAction _output_get actions))
  (bind _output_get_2 (LocalVariables|SetActionsLeft _actionsleft))
  ;[0.15 0.15 0.15 0.5] If actions still remain, begin incrementing actions on follow up scene blocks
  (if (>= _output_get_2 0)
    (while (and (>= (LocalVariables|GetActionsLeft) 0) (Utilities|IsValid (Variables|/Game/IWABO/Shared/Blueprints/DayStructure/BP_SceneBlock.BP_SceneBlock_C|GetNextBlock (Variables|Default|GetCurrentSceneBlock))))
      (|IncrementBlock))
    (Utilities|IsValid (LocalVariables|GetSceneBlock)
      (:Is%20Valid
        (if (!= (Variables|Default|GetCurrentSceneBlock) (LocalVariables|GetSceneBlock))
          (|LogSceneBlockUpdate)
          ;[0.15 0.15 0.15 0.5] Stop previous scene block, then start next block once done
          (Default|EndBlock (Variables|Default|GetCurrentSceneBlock))
          (bind _output_get_3 (Variables|Default|SetCurrentSceneBlock (LocalVariables|GetSceneBlock)))
          (Default|StartBlock _output_get_3 self))))))

(fn InitSceneBlocks
  (LocalVariables|SetNextBlock (Variables|/Game/IWABO/Shared/Blueprints/DayStructure/BP_SceneBlock.BP_SceneBlock_C|GetNextBlock (Variables|Default|GetCurrentSceneBlock)))
  (while (Utilities|IsValid (LocalVariables|GetNextBlock))
    (Utilities|IsValid (Variables|/Game/IWABO/Shared/Blueprints/DayStructure/BP_SceneBlock.BP_SceneBlock_C|GetDialogueInteractive (LocalVariables|GetNextBlock))
      (:Is%20Valid
        (Default|SetEnabled (Variables|/Game/IWABO/Shared/Blueprints/DayStructure/BP_SceneBlock.BP_SceneBlock_C|GetDialogueInteractive (LocalVariables|GetNextBlock)) false))
      (:Is%20Not%20Valid
        _))
    (LocalVariables|SetNextBlock (Variables|/Game/IWABO/Shared/Blueprints/DayStructure/BP_SceneBlock.BP_SceneBlock_C|GetNextBlock (LocalVariables|GetNextBlock)))))