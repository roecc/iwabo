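; BP_DialogueInteractive is an interactable actor that starts an Ink dialogue story when the player interacts with it.
; It caches the InkWrapper from BP_IwaboGameInstance on BeginPlay, then Interact begins the assigned Dialogue and, if a Cinematic is set, starts it through BP_ThirdPersonGameMode.
; Enter and exit handling only passes to the parent when a Dialogue is valid.
; UpdateDialogue and UpdateCinematic let other code swap the assigned content.
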(event EventBeginPlay
  (|CallParentFunction)
  (bind _asbp_iwabo_game_instance (Utilities|Casting|CastToBP_IwaboGameInstance (Game|GetGameInstance)))
  (Variables|Default|SetInkWrapper (Variables|/Game/IWABO/Core/Services/BP_IwaboGameInstance.BP_IwaboGameInstance_C|GetInkWrapper _asbp_iwabo_game_instance)))

(event Collision|EventActorBeginOverlap
  (params (OtherActor :type Actor%20Object%20Reference))
  (|CallParentFunction OtherActor) ; This node is disabled and will not be called.\nDrag off pins to build functionality.
)

(event EventTick
  (params (DeltaSeconds :type Float%20%28single-precision%29))
  (|CallParentFunction DeltaSeconds) ; This node is disabled and will not be called.\nDrag off pins to build functionality.
)

(event EventInteract
  (bind _cinematic (Variables|Default|GetCinematic))
  (Utilities|IsValid (Variables|Default|GetDialogue)
    (:Is%20Valid
      (Development|PrintText (Utilities|Text|ToText(String) (Utilities|String|Append "Beginning story " (Utilities|GetDisplayName (Variables|Default|GetDialogue)))))
      (Default|BeginStory (Variables|Default|GetInkWrapper) (Variables|Default|GetDialogue))
      (Utilities|IsValid _cinematic
        (:Is%20Valid
          (bind _asbp_third_person_game_mode (Utilities|Casting|CastToBP_ThirdPersonGameMode (Game|GetGameMode)))
          (Default|StartCinematic _asbp_third_person_game_mode _cinematic))))))

(event EventOnExit
  (Utilities|IsValid (Variables|Default|GetDialogue)
    (:Is%20Valid
      (|CallParentFunction))))

(event EventOnEnter
  (Utilities|IsValid (Variables|Default|GetDialogue)
    (:Is%20Valid
      (|CallParentFunction))))

(fn ConstructionScript
  (|CallParentFunction))

(fn UpdateDialogue
  (params (Dialogue :type Inkpot%20Story%20Asset%20Object%20Reference))
  (Variables|Default|SetDialogue Dialogue))

(fn UpdateCinematic
  (params (Cinematic :type Level%20Sequence%20Object%20Reference))
  (Variables|Default|SetCinematic Cinematic))