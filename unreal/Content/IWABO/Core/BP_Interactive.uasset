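; BP_Interactive is an interactive actor, apparently a base for objects the player can interact with, with an empty Interact event.
; It caches BP_ThirdPersonGameMode on BeginPlay, then uses that game mode's Prompt to display PromptText in OnEnter and hide it in OnExit.
; SetEnabled switches tick, visibility and collision together to turn the actor on or off.
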(event Custom|SetEnabled
  (params (bIsEnabled :type Boolean))
  (Actor|Tick|SetActorTickEnabled bIsEnabled)
  (Rendering|SetActorHiddenInGame (not bIsEnabled))
  (Collision|SetActorEnableCollision bIsEnabled))

(event EventBeginPlay
  (bind _asbp_third_person_game_mode (Utilities|Casting|CastToBP_ThirdPersonGameMode (Game|GetGameMode)))
  (Variables|Default|SetGameMode _asbp_third_person_game_mode))

(event Collision|EventActorBeginOverlap
  (params (OtherActor :type Actor%20Object%20Reference)))

(event EventInteract)

(event EventOnEnter
  (Default|Display (Variables|/Game/ThirdParty/UnrealTemplate/ThirdPerson/Blueprints/BP_ThirdPersonGameMode.BP_ThirdPersonGameMode_C|GetPrompt (Variables|Default|GetGameMode)) (Variables|Default|GetPromptText)))

(event EventOnExit
  (Default|Hide (Variables|/Game/ThirdParty/UnrealTemplate/ThirdPerson/Blueprints/BP_ThirdPersonGameMode.BP_ThirdPersonGameMode_C|GetPrompt (Variables|Default|GetGameMode))))

(fn ConstructionScript)