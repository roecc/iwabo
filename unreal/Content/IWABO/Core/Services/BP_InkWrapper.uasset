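; Service that bridges Inkpot Ink dialogue stories with the game's skill, state and config services, showing active stories on the story display.
; Choice and line tags are parsed by underscore-delimited prefix into typed tag data that applies mood and skill changes.
; Choice tags can also spend action points or roll skill checks into the Ink "outcome" variable, with a debug override.
; Ink external functions expose skill, mood and toxicity.
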(event Custom|OnStoryBegin
  (params (Story :type Inkpot%20Story%20Object%20Reference))
  (bind (_returnvalue _bsuccess) (Class|InkpotStory|GetBool Story "IsActive"))
  (|BindExternalFunctions Story)
  (|BindEvents Story)
  (if _bsuccess
    (if _returnvalue
      (Default|OnShowStory (Variables|Default|GetStoryDisplay) Story :!label _label)
      (else
        (Development|PrintString 0 "This is a passive conversation!!")))
    (else
      (goto _label))))

(event Custom|OnContinue
  (params (Story :type Inkpot%20Story%20Object%20Reference))
  (bind _data (CallFunction|GetTagData (Class|InkpotStory|GetCurrentTags Story)))
  (for _array_element _data
    (bind _asbp_update_mood_tag_data (Utilities|Casting|CastToBP_UpdateMoodTagData _array_element)
      (:then
        (Default|UpdateMood (Variables|Default|GetStateService) (Variables|/Game/IWABO/Core/Dialogues/BP_UpdateMoodTagData.BP_UpdateMoodTagData_C|GetCharacter _asbp_update_mood_tag_data) (Variables|/Game/IWABO/Core/Dialogues/BP_UpdateMoodTagData.BP_UpdateMoodTagData_C|GetAmount _asbp_update_mood_tag_data)))
      (:CastFailed
        (bind _asbp_update_skill_tag_data (Utilities|Casting|CastToBP_UpdateSkillTagData _array_element))
        (Default|UpdateSkillValue (Variables|Default|GetStateService) (Variables|/Game/IWABO/Core/Dialogues/BP_UpdateSkillTagData.BP_UpdateSkillTagData_C|GetSkill _asbp_update_skill_tag_data) (Variables|/Game/IWABO/Core/Dialogues/BP_UpdateSkillTagData.BP_UpdateSkillTagData_C|GetAmount _asbp_update_skill_tag_data))))))

(event Custom|OnMakeChoice
  (params (Story :type Inkpot%20Story%20Object%20Reference) (Choice :type Inkpot%20Choice%20Object%20Reference))
  (bind _data (CallFunction|GetTagData (Class|InkpotLine|GetTags Choice)))
  (for _array_element _data
    (bind _asbp_skill_check_tag_data (Utilities|Casting|CastToBP_SkillCheckTagData _array_element)
      (:then
        (|RollSkill Story _asbp_skill_check_tag_data))
      (:CastFailed
        (bind _asbp_use_action_tag_data (Utilities|Casting|CastToBP_UseActionTagData _array_element)
          (:then
            (|AddActions _asbp_use_action_tag_data))
          (:CastFailed
            (bind _asbp_update_mood_tag_data (Utilities|Casting|CastToBP_UpdateMoodTagData _array_element)
              (:then
                (Default|UpdateMood (Variables|Default|GetStateService) (Variables|/Game/IWABO/Core/Dialogues/BP_UpdateMoodTagData.BP_UpdateMoodTagData_C|GetCharacter _asbp_update_mood_tag_data) (Variables|/Game/IWABO/Core/Dialogues/BP_UpdateMoodTagData.BP_UpdateMoodTagData_C|GetAmount _asbp_update_mood_tag_data)))
              (:CastFailed
                (bind _asbp_update_skill_tag_data (Utilities|Casting|CastToBP_UpdateSkillTagData _array_element))
                (Default|UpdateSkillValue (Variables|Default|GetStateService) (Variables|/Game/IWABO/Core/Dialogues/BP_UpdateSkillTagData.BP_UpdateSkillTagData_C|GetSkill _asbp_update_skill_tag_data) (Variables|/Game/IWABO/Core/Dialogues/BP_UpdateSkillTagData.BP_UpdateSkillTagData_C|GetAmount _asbp_update_skill_tag_data))))))))))

(fn Init
  (params (SkillService :type BP%20Skill%20Service%20Object%20Reference) (StateService :type BP%20State%20Service%20Object%20Reference) (ConfigService :type BP%20Config%20Service%20Object%20Reference))
  (Variables|Default|SetStateService StateService)
  (Variables|Default|SetSkillService SkillService)
  (Variables|Default|SetConfigService ConfigService)
  (EventDispatchers|BindEventtoEventonStoryBegin (|Inkpot) (EventDispatchers|CreateEvent :!event Custom|OnStoryBegin)))

(fn BeginStory
  (params (StoryAsset :type Inkpot%20Story%20Asset%20Object%20Reference))
  (Class|Inkpot|BeginStory (|Inkpot) StoryAsset))

(fn UpdateOutcome
  (params (RollSkillData :type S%20Roll%20Skill%20Data%20Structure) (Story :type Inkpot%20Story%20Object%20Reference))
  (bind _makechoicedebugdata (Variables|Default|GetMakeChoiceDebugData))
  (bind (_bshouldoverrideskillcheck _boverride) (Utilities|Struct|BreakS_MakeChoiceDebugData _makechoicedebugdata))
  (if _bshouldoverrideskillcheck
    ;[0.15 0.15 0.15 0.5] If debug button was used, set outcome to override value in debug data
    (Class|InkpotStory|SetBool Story "outcome" _boverride)
    (Development|PrintText 0 (Utilities|Text|FormatText "DEBUG: Force override ink var \"outcome\" to {override}" _boverride))
    (elif (|ShouldUpdate RollSkillData)
      (bind _success (Default|RollSkill (Variables|Default|GetSkillService) RollSkillData))
      (Class|InkpotStory|SetBool Story "outcome" _success))))

(fn SetStoryDisplay
  (params (StoryDisplay :type WBP%20Display%20Object%20Reference))
  (Variables|Default|SetStoryDisplay StoryDisplay))

(fn GetTagData
  (params (Tags :type Array%20of%20Strings))
  (bind _array_element (Utilities|Array|ForEachLoopwithBreak Tags)
    (:LoopBody
      (if (> (Utilities|Array|Length (Utilities|String|ParseIntoArray _array_element "_")) 0)
        (switch string (Utilities|Array|Get(acopy) (Utilities|String|ParseIntoArray _array_element "_"))
          (:sc
            (if (not (LocalVariables|GetbHasSkillCheckTag))
              (bind _returnvalue (CallFunction|TryGetSkillCheckTagData (Utilities|String|ParseIntoArray _array_element "_") false))
              (Utilities|IsValid _returnvalue
                (:Is%20Valid
                  (LocalVariables|SetbHasSkillCheckTag true)
                  (Utilities|Array|Add (LocalVariables|GetTagDatas) _returnvalue)))))
          (:asc
            (if (not (LocalVariables|GetbHasSkillCheckTag))
              (bind _returnvalue_2 (CallFunction|TryGetSkillCheckTagData (Utilities|String|ParseIntoArray _array_element "_") true))
              (Utilities|IsValid _returnvalue_2
                (:Is%20Valid
                  (LocalVariables|SetbHasSkillCheckTag true)
                  (Utilities|Array|Add (LocalVariables|GetTagDatas) _returnvalue_2)))))
          (:ua
            (if (not (LocalVariables|GetbHasUseActionTag))
              (bind _returnvalue_3 (CallFunction|TryGetUseActionTagData (Utilities|String|ParseIntoArray _array_element "_")))
              (Utilities|IsValid _returnvalue_3
                (:Is%20Valid
                  (LocalVariables|SetbHasUseActionTag true)
                  (Utilities|Array|Add (LocalVariables|GetTagDatas) _returnvalue_3)))))
          (:um
            (bind _tagdata (CallFunction|TryGetUpdateMoodTagData (Utilities|String|ParseIntoArray _array_element "_")))
            (Utilities|IsValid _tagdata
              (:Is%20Valid
                (Utilities|Array|Add (LocalVariables|GetTagDatas) _tagdata))))
          (:us
            (bind _tagdata_2 (CallFunction|TryGetUpdateSkillTagData (Utilities|String|ParseIntoArray _array_element "_")))
            (Utilities|IsValid _tagdata_2
              (:Is%20Valid
                (Utilities|Array|Add (LocalVariables|GetTagDatas) _tagdata_2)))))))
    (:Completed
      (return (LocalVariables|GetTagDatas)))))

(fn TryGetSkillCheckTagData
  (params (TagComponents :type Array%20of%20Strings) (bRollAgainst :type Boolean))
  (bind _returnvalue (Utilities|Array|Length TagComponents))
  (bind _skill (|IsSkillConfigured TagComponents _returnvalue))
  (LocalVariables|SetSkill _skill)
  (|TryAddModifiers TagComponents _returnvalue)
  (bind _returnvalue_2 (Game|ConstructObjectfromClass "/Game/IWABO/Core/Dialogues/BP_SkillCheckTagData.BP_SkillCheckTagData_C"))
  (Variables|/Game/IWABO/Core/Dialogues/BP_SkillCheckTagData.BP_SkillCheckTagData_C|SetSkill _returnvalue_2 (LocalVariables|GetSkill))
  (Variables|/Game/IWABO/Core/Dialogues/BP_SkillCheckTagData.BP_SkillCheckTagData_C|SetModifier _returnvalue_2 (LocalVariables|GetModifiers))
  (Variables|/Game/IWABO/Core/Dialogues/BP_SkillCheckTagData.BP_SkillCheckTagData_C|SetbRollAgainst _returnvalue_2 bRollAgainst)
  (Variables|/Game/IWABO/Core/Dialogues/BP_InkChoiceTagData.BP_InkChoiceTagData_C|SetType _returnvalue_2 "NewEnumerator0")
  (return _returnvalue_2))

(fn TryGetUseActionTagData
  (params (TagComponents :type Array%20of%20Strings))
  (bind _output (Utilities|Array|Get(acopy) TagComponents 1))
  ;[0.15 0.15 0.15 0.5] Try get configured points
  (if (> (Utilities|Array|Length TagComponents) 1)
    ;[0.15 0.15 0.15 0.5] Try parse configured points
    (bind (_outvalue _returnvalue) (Class|IwaboBlueprintFunctionLibrary|TryParseInt _output))
    (if _returnvalue
      (bind _returnvalue_2 (Game|ConstructObjectfromClass "/Game/IWABO/Core/Dialogues/BP_UseActionTagData.BP_UseActionTagData_C"))
      (Variables|/Game/IWABO/Core/Dialogues/BP_UseActionTagData.BP_UseActionTagData_C|SetAmount _returnvalue_2 _outvalue)
      (Variables|/Game/IWABO/Core/Dialogues/BP_InkChoiceTagData.BP_InkChoiceTagData_C|SetType _returnvalue_2 "NewEnumerator1")
      (else
        (Development|PrintText 0 (Utilities|Text|FormatText "ERROR: Could not parse action point {point}!" (Utilities|Text|ToText(String) _output)))))
    (return _returnvalue_2)
    (else
      (Development|PrintText 0 (Utilities|Text|FormatText "ERROR: Dialogue choice is set to use an action but no points were configured!")))))

(fn TryGetUpdateMoodTagData
  (params (TagComponents :type Array%20of%20Strings))
  (bind _output_get (LocalVariables|SetComponentsLength (Utilities|Array|Length TagComponents)))
  ;[0.15 0.15 0.15 0.5] Try get configured character
  (if (> _output_get 1)
    (LocalVariables|SetCharacterAcronym (Utilities|Array|Get(acopy) TagComponents 1))
    (|GetCharacter)
    (if (> (LocalVariables|GetComponentsLength) 2)
      (|GetAmount TagComponents)
      (bind _returnvalue (Game|ConstructObjectfromClass "/Game/IWABO/Core/Dialogues/BP_UpdateMoodTagData.BP_UpdateMoodTagData_C"))
      (Variables|/Game/IWABO/Core/Dialogues/BP_UpdateMoodTagData.BP_UpdateMoodTagData_C|SetAmount _returnvalue (LocalVariables|GetAmount))
      (Variables|/Game/IWABO/Core/Dialogues/BP_UpdateMoodTagData.BP_UpdateMoodTagData_C|SetCharacter _returnvalue (LocalVariables|GetCharacter))
      (Variables|/Game/IWABO/Core/Dialogues/BP_InkChoiceTagData.BP_InkChoiceTagData_C|SetType _returnvalue "NewEnumerator2")
      (return _returnvalue)
      (else
        (|LogAmountMissingError)))
    (else
      (|LogCharacterMissingError))))

(fn TryGetUpdateSkillTagData
  (params (TagComponents :type Array%20of%20Strings))
  (bind _output_get (LocalVariables|SetComponentsLength (Utilities|Array|Length TagComponents)))
  ;[0.15 0.15 0.15 0.5] Try get configured skill
  (if (> _output_get 1)
    (LocalVariables|SetSkill (Utilities|Array|Get(acopy) TagComponents 1))
    (|GetSkill)
    (if (> (LocalVariables|GetComponentsLength) 2)
      (|GetSkillAmount TagComponents)
      (bind _returnvalue (Game|ConstructObjectfromClass "/Game/IWABO/Core/Dialogues/BP_UpdateSkillTagData.BP_UpdateSkillTagData_C"))
      (Variables|/Game/IWABO/Core/Dialogues/BP_UpdateSkillTagData.BP_UpdateSkillTagData_C|SetAmount _returnvalue (LocalVariables|GetAmount))
      (Variables|/Game/IWABO/Core/Dialogues/BP_UpdateSkillTagData.BP_UpdateSkillTagData_C|SetSkill _returnvalue (LocalVariables|GetSkill))
      (Variables|/Game/IWABO/Core/Dialogues/BP_InkChoiceTagData.BP_InkChoiceTagData_C|SetType _returnvalue "NewEnumerator3")
      (return _returnvalue)
      (else
        (|LogSkillAmountMissingError)))
    (else
      (|LogSkillMissingError))))

(fn ReadSkill
  (params (Values :type Array%20of%20Inkpot%20Value%20Structures))
  (bind _output (Utilities|Array|Get(acopy) Values))
  (bind _returnvalue (Class|InkpotValueLibrary|InkpotValueasString _output))
  (bind (_bvalid _skillstate) (Default|TryGetSkill (Variables|Default|GetStateService) _returnvalue))
  (if _bvalid
    (LocalVariables|SetSkillValue (.Value (Utilities|Struct|BreakSSkillState _skillstate)))
    (else
      (Development|PrintText 0 (Utilities|Text|FormatText "ERROR: Could not read skill {skill} from ink! Skill in invalid" _returnvalue))))
  (return (Class|InkpotValueLibrary|MakeIntInkpotValue (LocalVariables|GetSkillValue))))

(fn ReadMood
  (params (Values :type Array%20of%20Inkpot%20Value%20Structures))
  (bind _output (Utilities|Array|Get(acopy) Values))
  (bind _returnvalue (Class|InkpotValueLibrary|InkpotValueasString _output))
  (bind (_result _character _bvalid) (Default|GetCharacterConfigfromAcronym (Variables|Default|GetConfigService) _returnvalue))
  (if _bvalid
    (bind (_state _bisvalid) (Default|GetCharacterState (Variables|Default|GetStateService) _character))
    (if _bisvalid
      (return (Class|InkpotValueLibrary|MakeIntInkpotValue (.Mood (Utilities|Struct|BreakS_CharacterState _state))))
      (else
        (Development|PrintText 0 (Utilities|Text|FormatText "ERROR: Cannot read mood from ink as character acronym {acronym} has invalid state!" _returnvalue))))
    (else
      (Development|PrintText 0 (Utilities|Text|FormatText "ERROR: Cannot read mood from ink as character acronym {acronym} has invalid config!" _returnvalue)))))

(fn ReadIsSkillToxic
  (params (Values :type Array%20of%20Inkpot%20Value%20Structures))
  (bind _output (Utilities|Array|Get(acopy) Values))
  (bind _returnvalue (Class|InkpotValueLibrary|InkpotValueasString _output))
  (bind (_bvalid _skillstate) (Default|TryGetSkill (Variables|Default|GetStateService) _returnvalue))
  (if _bvalid
    (LocalVariables|SetbIsToxic (>= (.Value (Utilities|Struct|BreakSSkillState _skillstate)) (.ToxSwitch (Default|GetSkillConfig (Variables|Default|GetConfigService)))))
    (else
      (Development|PrintText 0 (Utilities|Text|FormatText "ERROR: Could not read skill {skill} isToxic from ink! Skill in invalid" _returnvalue))))
  (return (Class|InkpotValueLibrary|MakeBoolInkpotValue (LocalVariables|GetbIsToxic))))

(fn SetMakeChoiceDebugData
  (params (Data :type S%20Make%20Choice%20Debug%20Data%20Structure))
  (Variables|Default|SetMakeChoiceDebugData Data))