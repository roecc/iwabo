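; BP_IwaboGameInstance is the game instance for IWABO that creates and holds the game's core service objects.
; On Init it constructs the Config, State and Skill services in dependency order and stores each in a variable.
; The State service is initialized with the Config service, and the Skill service with the Skills data from the State service's state.
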(event EventInit
  (bind _returnvalue (Game|ConstructObjectfromClass "/Game/IWABO/Core/Services/Config/BP_ConfigService.BP_ConfigService_C"))
  (bind _output_get (Variables|Default|SetConfigService _returnvalue))
  (bind _returnvalue_2 (Game|ConstructObjectfromClass "/Game/IWABO/Core/Services/State/BP_StateService.BP_StateService_C"))
  (bind _output_get_2 (Variables|Default|SetStateService _returnvalue_2))
  (Default|Init _output_get_2 _output_get)
  (bind _returnvalue_3 (Game|ConstructObjectfromClass "/Game/IWABO/Core/Services/BP_SkillService.BP_SkillService_C"))
  (bind _output_get_3 (Variables|Default|SetSkillService _returnvalue_3))
  (Default|Init _output_get_3 (Variables|/Game/IWABO/Core/Services/State/BP_State.BP_State_C|GetSkills (Variables|/Game/IWABO/Core/Services/State/BP_StateService.BP_StateService_C|GetState (Variables|Default|GetStateService)))))