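; BP_StateService holds the game's state object and provides lookups for NPC state and skill values.
; Init stores the config service and constructs a default BP_State, a placeholder until state is loaded from disk.
; Lookups linearly search the state's Npcs and Skills arrays by character or Id, with no explicit not-found handling.
; Requesting NPC state for Daryl, the first character enum entry, only prints an error.
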(fn Init
  (params (ConfigService :type BP%20Config%20Service%20Object%20Reference))
  (bind _returnvalue (Game|ConstructObjectfromClass "/Game/IWABO/Core/Services/State/BP_State.BP_State_C")) ; For now we construct a default state object, but later this should be loaded from disk
  (Variables|Default|SetState _returnvalue)
  (Variables|Default|SetConfigService ConfigService))

(fn GetNpcState
  (params (Character :type ECharacterName%20Enum :default "NewEnumerator0"))
  (if (Utilities|Enum|Equal(Enum) Character "NewEnumerator0")
    (Development|PrintText 0 "Can't get NPC state for Daryl!")
    (else
      (bind _array_element (Utilities|Array|ForEachLoopwithBreak (Variables|/Game/IWABO/Core/Services/State/BP_State.BP_State_C|GetNpcs (Variables|Default|GetState)) :!label _label)
        (:LoopBody
          (if (Utilities|Enum|Equal(Enum) (.Character (Utilities|Struct|BreakSNpcState _array_element)) Character)
            (goto _label Break)))
        (:Completed
          (return _array_element))))))

(fn GetSkillValue
  (params (Id :type String))
  (bind _array_element (Utilities|Array|ForEachLoopwithBreak (Variables|/Game/IWABO/Core/Services/State/BP_State.BP_State_C|GetSkills (Variables|Default|GetState)) :!label _label)
    (:LoopBody
      (if (Utilities|Enum|Equal(Enum) (.Id (Utilities|Struct|BreakSSkillState _array_element)) Id)
        (goto _label Break)))
    (:Completed
      (return (.Value (Utilities|Struct|BreakSSkillState _array_element))))))