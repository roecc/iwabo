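; BP_ConfigService is a service that gives read-only access to game configuration held in a single Config variable.
; Getters return time settings (tick rate, hour length, day start and end, debug dilation speed) and skill settings (limits, ToxSwitch, starting skills).
; Starting skills are looked up by DefaultId with a linear search, and character configs by a map Find, neither reporting a failed match.
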(fn DebugGetTimeDilationSpeed
  (return (Variables|/Game/IWABO/Core/Services/Config/BP_Config.BP_Config_C|GetDebugTimeDilationSpeed (Variables|Default|GetConfig))))

(fn GetTicksPerHour
  (return (Variables|/Game/IWABO/Core/Services/Config/BP_Config.BP_Config_C|GetTicksPerHour (Variables|Default|GetConfig))))

(fn GetTimeConfig
  (bind _config (Variables|Default|GetConfig))
  (return (Variables|/Game/IWABO/Core/Services/Config/BP_Config.BP_Config_C|GetTicksPerHour _config) (Variables|/Game/IWABO/Core/Services/Config/BP_Config.BP_Config_C|GetSecondsPerHour _config) (Variables|/Game/IWABO/Core/Services/Config/BP_Config.BP_Config_C|GetStartTimeMinutes _config) (Variables|/Game/IWABO/Core/Services/Config/BP_Config.BP_Config_C|GetEndTimeMinutes _config)))

(fn GetSkillConfig
  (bind _config (Variables|Default|GetConfig))
  (return (Variables|/Game/IWABO/Core/Services/Config/BP_Config.BP_Config_C|GetMinSkill _config) (Variables|/Game/IWABO/Core/Services/Config/BP_Config.BP_Config_C|GetMaxSkill _config) (Variables|/Game/IWABO/Core/Services/Config/BP_Config.BP_Config_C|GetToxSwitch _config) (Variables|/Game/IWABO/Core/Services/Config/BP_Config.BP_Config_C|GetStartingSkills _config)))

(fn GetSkillConfigbyId
  (params (DefaultId :type String))
  (bind _array_element (Utilities|Array|ForEachLoopwithBreak (Variables|/Game/IWABO/Core/Services/Config/BP_Config.BP_Config_C|GetStartingSkills (Variables|Default|GetConfig)) :!label _label)
    (:LoopBody
      (if (Utilities|Enum|Equal(Enum) (.DefaultId (Utilities|Struct|BreakS_SkillConfig _array_element)) DefaultId)
        (goto _label Break)))
    (:Completed
      (return _array_element))))

(fn GetCharacterConfig
  (params (Character :type ECharacterName%20Enum :default "NewEnumerator0"))
  (return (.Value (Utilities|Map|Find (Variables|/Game/IWABO/Core/Services/Config/BP_Config.BP_Config_C|GetCharacters (Variables|Default|GetConfig)) Character))))