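; BP_SkillService is a service that resolves percentile skill checks against skills held in the StateService passed to Init.
; RollSkill sums modifiers and compares skill minus a 1–100 roll minus modifiers to zero, with RollAgainst inverting success.
; Each valid roll also nudges the stored skill up, or down when rolling against.
; It prints the result for debugging, or a warning for invalid skills.
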(fn Init
  (params (StateService :type BP%20State%20Service%20Object%20Reference))
  (Variables|Default|SetStateService StateService))

(fn RollSkill
  (params (Skill :type String) (Modifiers :type Array%20of%20Integers) (bRollAgainst :type Boolean))
  (bind _returnvalue (Math|Random|RandomIntegerinRange 1 100))
  (bind (_bvalid _skillstate) (Default|TryGetSkill (Variables|Default|GetStateService) Skill))
  (if _bvalid
    ;[0.15 0.15 0.15 0.5] Sum modifiers, save to Modifier Sum variable
    (for _array_element Modifiers
      (LocalVariables|SetModifierSum (+ _array_element (LocalVariables|GetModifierSum))))
    ;[0.15 0.15 0.15 0.5] Update skill in state
    (Default|UpdateSkillValue (Variables|Default|GetStateService) Skill (Math|Integer|SelectInt -1 1 bRollAgainst))
    ;[0.15 0.15 0.15 0.5] Debug Data
    (Development|PrintString 0 (Utilities|String|Append "Roll Skill:  " Skill ", Modifiers: " (Class|IwaboBlueprintFunctionLibrary|IntArraytoString Modifiers true) ", Dice: " (Utilities|String|ToString(Integer) _returnvalue) ", Result: " (Utilities|String|SelectString "SUCCESS" "FAIL" (or (and (>= (|((skill-roll)-mods) (.Value (Utilities|Struct|BreakSSkillState _skillstate)) _returnvalue (LocalVariables|GetModifierSum)) 0) (not bRollAgainst)) (and bRollAgainst (< (|((skill-roll)-mods) (.Value (Utilities|Struct|BreakSSkillState _skillstate)) _returnvalue (LocalVariables|GetModifierSum)) 0)))) ", " (Utilities|String|ToString(Integer) (|((skill-roll)-mods) (.Value (Utilities|Struct|BreakSSkillState _skillstate)) _returnvalue (LocalVariables|GetModifierSum)))) true true "(R=0.000000,G=0.660000,B=1.000000,A=1.000000)" 2e+02)
    (return (or (and (>= (|((skill-roll)-mods) (.Value (Utilities|Struct|BreakSSkillState _skillstate)) _returnvalue (LocalVariables|GetModifierSum)) 0) (not bRollAgainst)) (and bRollAgainst (< (|((skill-roll)-mods) (.Value (Utilities|Struct|BreakSSkillState _skillstate)) _returnvalue (LocalVariables|GetModifierSum)) 0))))
    (else
      ;[0.15 0.15 0.15 0.5] Log warning and do nothing if skill invalid
      (Development|PrintText 0 (Utilities|Text|FormatText "Skill {skill} is invalid! Could not roll skill" Skill)))))