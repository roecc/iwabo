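; BP_SkillCheckTagData is a dialogue data Blueprint for skill checks that holds a list of modifiers.
; GetValidModifiers filters that list against game state flags read from the supplied StateService.
; A modifier counts as valid when its flag is empty or that flag is set, and the function returns the matching entries.
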(fn GetValidModifiers
  (params (StateService :type BP%20State%20Service%20Object%20Reference))
  (for _array_element (Variables|Default|GetModifiers)
    (if (Utilities|Array|IsEmpty (.Flag (Utilities|Struct|BreakS_SkillCheckModifierData _array_element)))
      (Utilities|Array|Add (LocalVariables|GetValidModifiers) _array_element :!label _label)
      (else
        (bind _result (Default|GetFlag StateService (.Flag (Utilities|Struct|BreakS_SkillCheckModifierData _array_element))))
        (if _result
          (goto _label)))))
  (return (LocalVariables|GetValidModifiers)))